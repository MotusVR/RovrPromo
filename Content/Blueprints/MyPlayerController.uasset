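; Player controller that manages map changes, player pawn spawning and the UI flow from registration and info screens to lobby, loading and session menus.
; An HMD flag from BP_GameInstance routes lobby and loading widgets to the pawn's world-space widget window in VR, otherwise to the viewport.
; ChangeLevelMap swaps streamed levels, records the current one on the game instance and re-zeroes VR yaw.
; Older level-switch and menu-toggle logic remains unconnected.
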(event `self.ReceiveBeginPlay`
  (bind _asbp_game_instance (cast `/Game/Blueprints/BP_GameInstance` (`GameplayStatics.GetGameInstance`)))
  (set `self.PlayerControllerHMDCheck` (`/Game/Blueprints/BP_GameInstance.HMDCheck` _asbp_game_instance)))

(event `self.ChangeLevelMap`
  (params (NewMapName :type String))
  (bind _returnvalue (`KismetStringLibrary.Conv_StringToName` NewMapName))
  (bind _playerpawn (`self.PlayerPawn`))
  (bind _asbp_game_instance (cast `/Game/Blueprints/BP_GameInstance` (`GameplayStatics.GetGameInstance`) :!pure true))
  (bind (_returnvalue_roll _returnvalue_pitch _returnvalue_yaw) (`KismetMathLibrary.BreakRotator` (`SceneComponent.K2_GetComponentRotation` (`/Game/ThirdPersonBP/Blueprints/playerPawn.Camera` _playerpawn))))
  ;[1 1 1] Change LevelMap using Load and Unload StreamLevel
  (`GameplayStatics.LoadStreamLevel` _returnvalue true)
  (`GameplayStatics.UnloadStreamLevel` (`KismetStringLibrary.Conv_StringToName` (`/Game/Blueprints/BP_GameInstance.CurrentLoadedLevel` _asbp_game_instance)))
  (set `/Game/Blueprints/BP_GameInstance.CurrentLoadedLevel` (`KismetStringLibrary.Conv_NameToString` _returnvalue) _asbp_game_instance)
  (if (`self.PlayerControllerHMDCheck`)
    (`SceneComponent.K2_AddWorldRotation` (`/Game/ThirdPersonBP/Blueprints/playerPawn.VRParent` _playerpawn) (`KismetMathLibrary.MakeRotator` 0.0 0.0 (* -1 _returnvalue_yaw)) false false)))

(event `self.ReceiveTick`
  (params (DeltaSeconds :type "Float (single-precision)")))

(fn `Clear UI`
  (if (`self.PlayerControllerHMDCheck`)
    (`WidgetComponent.SetWidget` (`/Game/ThirdPersonBP/Blueprints/playerPawn.Widget_Window` (`self.PlayerPawn`)) null)
    (else
      (`WidgetLayoutLibrary.RemoveAllWidgets`))))

(fn `Create Info`
  (bind _returnvalue (`|CreateWidget` "/Game/UI/Login/ROVRInfo.ROVRInfo_C" self))
  (bind _output_get (set `self.ROVRInfo` _returnvalue))
  (`UserWidget.AddToViewport` _output_get 0))

(fn `Create Register`
  (bind _returnvalue (`|CreateWidget` "/Game/UI/Login/Register.Register_C" self))
  (bind _output_get (set `self.RegisterWB` _returnvalue))
  (`UserWidget.AddToViewport` _output_get 0))

(fn `Create Session Menu`
  (params (VideoVolume :type "Float (double-precision)") (MusicVolume :type "Float (double-precision)") (CGI_Scene :type Boolean))
  (bind _loadingwidget (`self.LoadingWidget`))
  (`/Engine/EditorBlueprintResources/StandardMacros.IsValid` _loadingwidget
    (:`Is Valid`
      (`Widget.RemoveFromParent` _loadingwidget))
    (:`Is Not Valid`
      _))
  (if (not (`self.PlayerControllerHMDCheck`))
    (bind _returnvalue (`|CreateWidget` "/Game/UI/Session/SessionMenu.SessionMenu_C" self VideoVolume MusicVolume CGI_Scene))
    (bind _output_get (set `self.SessionMenu` _returnvalue))
    (`UserWidget.AddToViewport` _output_get 0)))

(fn `CreateLobbyMenu`
  (returns (LobbyMenu :type "/Game/UI/Lobby/LobbyMenu Object Reference"))
  (bind _lobbymenu (`self.LobbyMenu`))
  (bind _sessionmenu (`self.SessionMenu`))
  (`/Engine/EditorBlueprintResources/StandardMacros.IsValid` _sessionmenu
    (:`Is Valid`
      (`Widget.RemoveFromParent` _sessionmenu))
    (:`Is Not Valid`
      _))
  (`/Engine/EditorBlueprintResources/StandardMacros.IsValid` (`self.LobbyMenu`)
    (:`Is Valid`
      _)
    (:`Is Not Valid`
      (bind _returnvalue (`|CreateWidget` "/Game/UI/Lobby/LobbyMenu.LobbyMenu_C" self))
      (set `self.LobbyMenu` _returnvalue)))
  ;[1 1 1] Do android menu handling
  (if (`self.PlayerControllerHMDCheck`)
    (`WidgetComponent.SetWidget` (`/Game/ThirdPersonBP/Blueprints/playerPawn.Widget_Window` (`self.PlayerPawn`)) _lobbymenu)
    (`/Game/UI/Lobby/LobbyMenu.SetMenuScroll` _lobbymenu 0.0)
    (else
      (`UserWidget.AddToViewport` (`self.LobbyMenu`) 0)))
  (return (`self.LobbyMenu`)))

(fn `CreatePlayerPawn`
  (params (`Spawn Transform Location` :type "Vector Structure") (`Spawn Transform Rotation` :type "Rotator Structure"))
  (returns (PlayerPawn1 :type "/Game/ThirdPersonBP/Blueprints/playerPawn Object Reference"))
  (bind _returnvalue (`self.K2_GetPawn`))
  (bind _playerpawn (`self.PlayerPawn`))
  (bind _camera (`/Game/ThirdPersonBP/Blueprints/playerPawn.Camera` (`self.PlayerPawn`)))
  (`/Engine/EditorBlueprintResources/StandardMacros.IsValid` _returnvalue
    (:`Is Valid`
      (`self.K2_DestroyActor` _returnvalue))
    (:`Is Not Valid`
      _))
  (bind _returnvalue_2 (`|SpawnActorFromClass` "/Game/ThirdPersonBP/Blueprints/playerPawn.playerPawn_C" (`KismetMathLibrary.MakeTransform` `Spawn Transform Location` `Spawn Transform Rotation`) "AdjustIfPossibleButAlwaysSpawn" "OverrideRootScale" self null))
  (set `self.PlayerPawn` _returnvalue_2)
  (if (== (`HeadMountedDisplayFunctionLibrary.GetHMDDeviceName`) "FPicoVRHMD")
    (set `CameraComponent.bUsePawnControlRotation` true _camera)
    (else
      (set `CameraComponent.bUsePawnControlRotation` false _camera)))
  (`self.Possess` _playerpawn)
  (return _playerpawn))

(fn `GetPlayerStarts`
  (returns (PlayerStarts :type "Array of PlayerStart Object Reference"))
  (bind _outactors (`GameplayStatics.GetAllActorsOfClass` "/Script/Engine.PlayerStart"))
  (return _outactors))

(fn `HideLoadingScreen`
  (bind _loadingwidget (`self.LoadingWidget`))
  (`KismetSystemLibrary.PrintString` "Hide Loading")
  (`/Engine/EditorBlueprintResources/StandardMacros.IsValid` _loadingwidget
    (:`Is Valid`
      (`Widget.RemoveFromParent` _loadingwidget))
    (:`Is Not Valid`
      (`KismetSystemLibrary.PrintString` "Not valid" true true (struct :`R` 1.0 :`A` 1.0)))))

(fn `InfoOKButtonPressed`
  (`Widget.RemoveFromParent` (`self.ROVRInfo`))
  (`self.ChangeLevelMap` (cast `/Game/Blueprints/IGameModeChange_BP` self :!pure true) "LobbyMap"))

(fn `QuitGame`
  (`KismetSystemLibrary.QuitGame` null "Quit"))

(fn `ResetGame`
  (bind _returnvalue (`GameplayStatics.GetCurrentLevelName` true))
  (`GameplayStatics.OpenLevel` (`KismetStringLibrary.Conv_StringToName` _returnvalue)))

(fn `ResetVolumeLevels`
  (`/Game/Blueprints/BP_GameInstance.ResetVolumeLevels` (`self.As Playfab Instance`)))

(fn `SetDialogMessage`
  (params (TitleText :type String) (MessageText :type String))
  (locals (DialogBox :type "/Game/UI/Login/DialogBox Object Reference"))
  (`/Game/UI/Login/Register.SetDialogMessage` (`self.RegisterWB`) TitleText MessageText))

(fn `ShowCloseGameDialog`
  (`|CreateWidget` "/Game/UI/AllLevels/CloseGameDialog.CloseGameDialog_C" self))

(fn `ShowLoadingScreen`
  (bind _lobbymenu (`self.LobbyMenu`))
  (`/Engine/EditorBlueprintResources/StandardMacros.IsValid` _lobbymenu
    (:`Is Valid`
      (`Widget.RemoveFromParent` _lobbymenu))
    (:`Is Not Valid`
      _))
  (bind _returnvalue (`|CreateWidget` "/Game/UI/AllLevels/LoadingScreen.LoadingScreen_C" self))
  (set `self.LoadingWidget` _returnvalue)
  ;[1 1 1] Do android menu handling
  (if (`self.PlayerControllerHMDCheck`)
    (`WidgetComponent.SetWidget` (`/Game/ThirdPersonBP/Blueprints/playerPawn.Widget_Window` (`self.PlayerPawn`)) (`self.LoadingWidget`))
    (else
      (`UserWidget.AddToViewport` (`self.LoadingWidget`) 0))))

(fn `SubmitButtonPressed`
  (`Widget.RemoveFromParent` (`self.RegisterWB`))
  (`self.Create Info`))

(fn `UserConstructionScript`
  (bind _asbp_game_instance (cast `/Game/Blueprints/BP_GameInstance` (`GameplayStatics.GetGameInstance`)))
  (set `self.As Playfab Instance` _asbp_game_instance))