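; MySQL connector actor, based on a query demo, that opens a Care Show Database connection at BeginPlay using hardcoded server credentials.
; Events run select, single or batched update queries on connection 0, storing the latest query ID.
; Status callbacks print connection and update results, and forward select results to the query widget if valid.
; Widget creation and binding, the sample INSERT and update-status forwarding to the widget are disconnected.
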(event `self.ReceiveBeginPlay`
  (`self.CreateNewConnection` "92.205.6.97" "Care Show Database" "testClient" "Csbroadshow1!" (`self.Extra Params`)))

(event `self.OnConnectionStateChanged`
  (params (ConnectionStatus :type Boolean) (ConnectionID :type Integer) (ErrorMessage :type String))
  ;[1 1 1] On ConnectionStateChanged
  (if ConnectionStatus
    (`KismetSystemLibrary.PrintString` "Connection successful" true true (struct :`G` 1.0 :`A` 1.0) 5.0)
    (else
      (`KismetSystemLibrary.PrintString` "Connection failed" true true (struct :`R` 1.0 :`A` 1.0) 5.0)
      (`KismetSystemLibrary.PrintString` (`KismetStringLibrary.Concat_StrStr` "Error message: " ErrorMessage) true true (struct :`G` 0.66 :`B` 1.0 :`A` 1.0) 15.0))))

(event `OnCallSelectQuery`
  (params (Query :type String) (QueryID :type Integer))
  ;[1 1 1] Simple Query Execution
  ;;[0 0.2 0.54] This is Basic Query Demo. Plug this in to test out storing and retrieving data from Database
  ;;;[1 1 1] Select Query
  (`self.SelectDataFromQuery` 0 Query)
  (set `self.CurrentQueryID` QueryID))

(event `OnCallUpdateQuery`
  (params (UpdateQuery :type String) (QueryID :type Integer))
  ;[1 1 1] Simple Query Execution
  ;;[0 0.2 0.54] This is Basic Query Demo. Plug this in to test out storing and retrieving data from Database
  ;;;[1 1 1] Update Query
  (`self.UpdateDataFromQuery` 0 UpdateQuery)
  (set `self.CurrentQueryID` QueryID))

(event `OnUpdateMultipleQueries`
  (params (UpdateQueries :type "Array of String (by ref)") (QueryID :type Integer))
  ;[1 1 1] Simple Query Execution
  ;;[0 0.2 0.54] This is Basic Query Demo. Plug this in to test out storing and retrieving data from Database
  ;;;[0.1475 0 1] Update Multiple Queries at Once
  (`self.UpdateDataFromMultipleQueries` 0 UpdateQueries)
  (set `self.CurrentQueryID` QueryID))

(event `OnCloseConnection`
  (bind _dbconnectionwidget (`self.DBConnectionWidget`))
  ;[1 1 1] Simple Query Execution
  ;;[0 0.2 0.54] This is Basic Query Demo. Plug this in to test out storing and retrieving data from Database
  ;;;[0.1504 0 1] Close Connection
  (`self.CloseConnection` 0)
  (`/Engine/EditorBlueprintResources/StandardMacros.IsValid` _dbconnectionwidget
    (:`Is Valid`
      (`UserWidget.AddToViewport` _dbconnectionwidget 0)
      (`/MySQL/Widgets/UMG_DBConnection.ResetWidget` _dbconnectionwidget))))

(event `self.OnQueryUpdateStatusChanged`
  (params (IsSuccessful :type Boolean) (ErrorMessage :type String))
  ;[1 1 1] Simple Query Execution
  ;;[1 1 1] On Query Update Status Changed
  (`KismetSystemLibrary.PrintString` (`KismetStringLibrary.Concat_StrStr` "Update successful: " (`KismetStringLibrary.Conv_BoolToString` IsSuccessful) " \n" ErrorMessage) true true (struct :`G` 0.66 :`B` 1.0 :`A` 1.0) 10.0))

(event `self.OnQuerySelectStatusChanged`
  (params (IsSuccessful :type Boolean) (ErrorMessage :type String) (ResultByColumn :type "Array of MySQLDataTable Structure (by ref)") (ResultByRow :type "Array of MySQLDataRow Structure (by ref)"))
  ;[1 1 1] Simple Query Execution
  ;;[1 1 1] On Query Select Status Changed
  (`/Engine/EditorBlueprintResources/StandardMacros.IsValid` (`self.MySQLQueryWidget`)
    (:`Is Valid`
      (`/MySQL/Widgets/Umg_BasicQueryDemo.On SelectionStatus Changes` (`self.MySQLQueryWidget`) IsSuccessful ErrorMessage (`self.CurrentQueryID`) ResultByColumn ResultByRow))))

(fn `UserConstructionScript`)