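; Photon Cloud networking object that pairs a VR headset client with a non-HMD client for shared map and media sessions.
; On init it binds Photon callbacks, pings regions and starts login, then drives menus and room join/leave.
; The master's StartGame writes map, video and volumes into custom room properties, which receivers apply through PlayerController.
; The headset streams camera rotation unreliably on a timer, sending only changes, for the non-HMD pawn to mirror.
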(event `On Player wants to connect from HUD`
  ;[1 1 1] CONNECT - Button
  (`self.Connect`))

(event `Fake Begin Play`
  ;[1 1 1] Connect EVENT will come from this HUD
  (set `self.PlayerController` (cast `/Game/Blueprints/MyPlayerController` (`PhotonCloudAPIBPLibrary.GetFirstLocalPlayerController` self) :!pure true))
  (bind _playerpawn1 (`/Game/Blueprints/MyPlayerController.CreatePlayerPawn` :`self` (`self.PlayerController`) :`Spawn Transform Location` (`Actor.K2_GetActorLocation` (`|GetArrayItem` (`/Game/Blueprints/MyPlayerController.GetPlayerStarts` (`self.PlayerController`))))))
  (set `self.MyPlayerPawn` _playerpawn1)
  (`/Game/Blueprints/MyPlayerController.StartLoginProcess` (`self.PlayerController`)))

(event `On Photon Connection Error` :!signature `self.OnPhotonConnectionError`
  (params (ErrorCode :type "EPhotonErrorCode Enum" :default "OK") (ErrorMessage :type String))
  ;[1 1 1] ON DISCONNECTION
  (`KismetSystemLibrary.PrintString` null ErrorMessage true true (struct :`R` 1.0 :`A` 1.0) 10.0)
  (switch `EPhotonErrorCode` ErrorCode
    (:`OK`
      _)
    (:`OPERATION_DENIED`
      _)
    (:`OPERATION_INVALID`
      _)
    (:`INTERNAL_SERVER_ERROR`
      _)
    (:`INVALID_AUTHENTICATION`
      _)
    (:`SERVER_FULL`
      _)
    (:`USER_BLOCKED`
      _)
    (:`INVALID_REGION`
      _)
    (:`CUSTOM_AUTHENTICATION_FAILED`
      _)
    (:`AUTHENTICATION_TOKEN_EXPIRED`
      _)
    (:`INVALID_ENCRYPTION_PARAMETERS`
      _))
  (`KismetSystemLibrary.PrintString` self ErrorMessage))

(event `HandleLeaveRoom`
  (bind _lobbyui (`self.LobbyUI`))
  ;[1 1 1] Handles clean up when leaving the room
  (`/Engine/EditorBlueprintResources/StandardMacros.IsValid` _lobbyui
    (:`Is Valid`
      (`Widget.RemoveFromParent` _lobbyui))
    (:`Is Not Valid`
      _))
  (`/Game/Blueprints/MyPlayerController.ShowMotionController` (`self.PlayerController`))
  (`self.JoinLobbyRoom` ""))

(event `Send My player location and rotation`
  (bind _returnvalue (`SceneComponent.K2_GetComponentRotation` (`/Game/ThirdPersonBP/Blueprints/playerPawn.Camera` (`self.MyPlayerPawn`))))
  ;[1 1 1] LOCAL PLAYER
  ;;[1 0.1499 0.6604] SEND MY PLAYER LOCATION AND ROTATION
  (if (!= (`self.LastPlayerRotation`) _returnvalue :`ErrorTolerance` 0.1)
    (bind _output_get (set `self.LastPlayerRotation` _returnvalue))
    (`self.SendPlayerLocationRotation` :`Location` (`self.DefaultLocation`) :`Rotation` _output_get :`Reliable` false)))

(event `On Photon Cloud Event Changed`
  (params (NewState :type "EPhotonCloudStates Enum" :default "UNINITIALIZED"))
  ;[1 1 1] PHOTON CLOUD STATE CHANGED
  (`KismetSystemLibrary.PrintString` self (`|GetEnumeratorNameAsString` NewState) true true (struct :`G` 1.0 :`A` 1.0) 10.0)
  (switch `EPhotonCloudStates` NewState
    (:`PEERCREATED`
      (`self.ReConnect`))
    (:`JOINEDLOBBY`
      (`self.OnPlayerJoinedLobbyRoom`))
    (:`JOINED`
      (`KismetSystemLibrary.PrintString` self (`KismetStringLibrary.Concat_StrStr` "JOINED ROOM --> " (`self.GetRoomName`)) true true (struct :`R` 1.0 :`B` 0.814345 :`A` 1.0)))
    (:`LEFT`
      (`KismetSystemLibrary.PrintString` self "LEFT ROOM"))))

(event `CustomLeaveRoom`
  ;[1 1 1] Handles leaving the room - moving to main menu map and displaying menu
  (`self.HandleLeaveRoom`)
  (`self.LeaveRoom` false))

(event `self.OnPhotonCloudInitialized`
  (`|ExecutionSequence`
    (:`then_0`
      (`KismetSystemLibrary.K2_SetTimerDelegate` (delegate `Fake Begin Play`) 1.1)
      ;[1 1 1] ON DISCONNECTION
      (add `self.OnPhotonConnectionError` (delegate `On Photon Connection Error`)))
    (:`then_1`
      ;[1 1 1] PHOTON CLOUD STATE CHANGED
      (add `self.OnPhotonCloudStateChanged` (delegate `On Photon Cloud Event Changed`)))
    (:`then_2`
      (add `self.OnPlayerJoinedRoom` (delegate `On Player Joined`)))
    (:`then_3`
      (`self.Get Regions Pings`))
    (:`then_4`
      (add `self.OnPlayerJoinedLobbyRoom` (delegate `On Joined Lobby Room`))
      (add `self.OnJoinOrCreateRoomError` (delegate `Joining or Creating Room Error`)))
    (:`then_5`
      ;[0.4452 0.2195 0] PLAYER LEFT THE ROOM
      (add `self.OnPlayerLeftRoom` (delegate `Player Left Room`)))
    (:`then_6`
      (add `self.OnReceivedPlayerLocationRotation3d` (delegate `On Received new Player Location and Rotation`)))
    (:`then_7`
      (add `self.OnPlayerCustomPropertiesChanged` (delegate `On Player Custom Properties changed`)))
    (:`then_8`
      (add `self.OnPlayerColorChanged` (delegate `On Player Color Changed`)))
    (:`then_9`
      (add `self.OnReceivedPlayerData` (delegate `Received Player Data Event`)))
    (:`then_10`
      (add `self.OnReceivedChangedCustomRoomProperties` (delegate `On Custom Room Properties Arrive`)))
    (:`then_11`
      (add `self.OnUpdateRoomList` (delegate `On Room List Arrives`)))
    (:`then_12`
      (add `self.OnMasterChanged` (delegate `OnMasterChanged_Func`)))))

(event `On Player Joined` :!signature `self.OnPlayerJoinedRoom`
  (params (PlayerNumber :type Integer) (PlayerName :type String) (IsLocalPlayer :type Boolean))
  (bind _playercontroller (`self.PlayerController`))
  (bind _playercontroller_2 (`self.PlayerController`))
  (bind _lobbyui (`self.LobbyUI`))
  (bind _returnvalue (> (`self.GetCountPlayersInRoom`) 1))
  (bind _playercontrollerhmdcheck (`/Game/Blueprints/MyPlayerController.PlayerControllerHMDCheck` (`self.PlayerController`)))
  ;[1 1 1] PLAYER JOINED
  (`/Game/Blueprints/MyPlayerController.ResetVolumeLevels` _playercontroller)
  (`/Game/Blueprints/MyPlayerController.Get Enabled Videos` _playercontroller _returnvalue)
  (`/Game/Blueprints/MyPlayerController.Get Enabled AudioTracks` _playercontroller _returnvalue)
  (if IsLocalPlayer
    (`/Game/Blueprints/MyPlayerController.HideMotionController` _playercontroller_2)
    (`/Game/Blueprints/IGameModeChange_BP.ChangeLevelMap` (cast `/Game/Blueprints/IGameModeChange_BP` _playercontroller_2 :!pure true) (`PhotonJSON.GetString` (`self.GetCustomRoomProperties`) "mapName"))
    (`Widget.RemoveFromParent` (`self.MainMenuUI`))
    (`KismetSystemLibrary.PrintString` self (`KismetStringLibrary.Concat_StrStr` "Player " PlayerName " joined the room"))
    ;[1 1 1] SPAWN AND ADD PLAYER TO THE LIST OF PLAYERS
    (if (`KismetStringLibrary.EqualEqual_StrStr` (`PhotonJSON.GetString` (`self.GetCustomRoomProperties`) "mapName") "LobbyMap")
      (`/Engine/EditorBlueprintResources/StandardMacros.IsValid` _lobbyui
        (:`Is Valid`
          (`Widget.RemoveFromParent` _lobbyui))
        (:`Is Not Valid`
          _))
      (bind _lobbymenu (`/Game/Blueprints/MyPlayerController.CreateLobbyMenu` (`self.PlayerController`)))
      (bind _output_get (set `self.LobbyUI` _lobbymenu))
      (if _playercontrollerhmdcheck
        (`/Game/UI/Lobby/LobbyMenu.RemoveHeadsetConnected` _output_get)
        ;[1 1 1] LOCAL PLAYER
        (`|ExecutionSequence` :!label _label
          (:`then_0`
            ;;[1 1 1] Cache location and rotation
            (set `self.LastPlayerRotation` (`SceneComponent.K2_GetComponentRotation` (`/Game/ThirdPersonBP/Blueprints/playerPawn.Camera` (`self.MyPlayerPawn`)))))
          (:`then_1`
            ;;[1 0.1499 0.6604] SEND MY PLAYER LOCATION AND ROTATION
            (`KismetSystemLibrary.K2_SetTimerDelegate` (delegate `Send My player location and rotation`) 0.01 true 0.1))
          (:`then_2`
            (`/Game/Blueprints/MyPlayerController.HideLoadingScreen` (`self.PlayerController`))))
        (else
          (`KismetSystemLibrary.PrintString` null (`KismetStringLibrary.Conv_BoolToString` _playercontrollerhmdcheck) true true (struct :`R` 1.0 :`A` 1.0) 20.0)))
      (elif (`/Game/Blueprints/MyPlayerController.PlayerControllerHMDCheck` (`self.PlayerController`))
        (goto _label)))
    (elif (and (`self.AmIMaster`) (not IsLocalPlayer))
      (`/Game/UI/Lobby/LobbyMenu.HeadsetConnected` (`self.LobbyUI`)))))

(event `StartGame`
  (params (MapName :type Name) (VideoName :type String) (VideoVolume :type "Float (double-precision)") (MusicVolume :type "Float (double-precision)"))
  (bind _playercontroller (`self.PlayerController`))
  (bind _returnvalue (`KismetStringLibrary.Conv_NameToString` (`self.Map Name`)))
  ;[1 1 1] MATCHMAKING: Once all players are here in LobbyMap, go to forest and change the game mode in room properties.
  (bind _output_get (set `self.Map Name` MapName))
  (if (and (`self.AmIMaster`) (`KismetStringLibrary.NotEqual_StrStr` (`KismetStringLibrary.Conv_NameToString` _output_get) (`PhotonJSON.GetString` (`self.GetCustomRoomProperties`) "mapName")))
    (bind _returnvalue_2 (`PhotonJSON.SetString` (`PhotonJSON.Create` self) "mapName" (`KismetStringLibrary.Conv_NameToString` (`self.Map Name`))))
    (bind _output_get_2 (set `self.GameMode` 1))
    (bind _returnvalue_3 (`PhotonJSON.SetInteger` _returnvalue_2 "GameMode" _output_get_2))
    (bind _returnvalue_4 (`PhotonJSON.SetString` _returnvalue_3 "VideoName" VideoName))
    (bind _returnvalue_5 (`PhotonJSON.SetFloat` _returnvalue_4 "VideoVolume" VideoVolume))
    (bind _returnvalue_6 (`PhotonJSON.SetFloat` _returnvalue_5 "MusicVolume" MusicVolume))
    (`self.AddCustomRoomProperties` _returnvalue_6)
    (`/Game/Blueprints/IGameModeChange_BP.ChangeLevelMap` (cast `/Game/Blueprints/IGameModeChange_BP` _playercontroller :!pure true) _returnvalue)
    (if (not (`KismetStringLibrary.EqualEqual_StrStr` _returnvalue "LobbyMap"))
      (`/Game/Blueprints/MyPlayerController.ShowLoadingScreen` _playercontroller))))

(event `On Connect`)

(event `Joining or Creating Room Error` :!signature `self.OnJoinOrCreateRoomError`
  (params (ErrorCode :type "EPhotonErrorCode Enum" :default "OK") (ErrorMessage :type String))
  ;[1 0 0] ERROR : If there is no room
  (`KismetSystemLibrary.PrintString` null ErrorMessage true true (struct :`R` 1.0 :`A` 1.0) 10.0)
  (switch `EPhotonErrorCode` ErrorCode))

(event `On Joined Lobby Room`
  ;[1 0.6933 0.225] Once connected to photon, set my player name, list rooms, just join or create a room
  (`/Game/Blueprints/MyPlayerController.HideLoggingInScreen` (`self.PlayerController`))
  (set `self.MainMenuUI` (`/Game/Blueprints/MyPlayerController.CreateMainMenu` (`self.PlayerController`)))
  (`/Game/Blueprints/IGameModeChange_BP.ChangeLevelMap` (cast `/Game/Blueprints/IGameModeChange_BP` (`self.PlayerController`) :!pure true) "MainMenuMap"))

(event `Player Left Room` :!signature `self.OnPlayerLeftRoom`
  (params (PlayerNumber :type Integer))
  (bind _playercontroller (`self.PlayerController`))
  (bind _returnvalue (> (`self.GetCountPlayersInRoom`) 1))
  ;[0.4452 0.2195 0] PLAYER LEFT THE ROOM
  (if (== -1 (`self.GetPlayerNumber`))
    _
    (elif (`/Game/Blueprints/MyPlayerController.PlayerControllerHMDCheck` (`self.PlayerController`))
      (`/Game/Blueprints/MyPlayerController.QuitGame` (`self.PlayerController`))
      (else
        (`/Game/UI/Lobby/LobbyMenu.HeadsetDisconnected` (`self.LobbyUI`))
        (`/Game/Blueprints/MyPlayerController.Get Enabled Videos` _playercontroller _returnvalue)
        (`/Game/Blueprints/MyPlayerController.UpdateVideos` _playercontroller)
        (`/Game/Blueprints/MyPlayerController.Get Enabled AudioTracks` _playercontroller _returnvalue)))))

(event `On Received new Player Location and Rotation` :!signature `self.OnReceivedPlayerLocationRotation3d`
  (params (PlayerNumber :type Integer) (Location :type "Vector Structure (by ref)") (Rotation :type "Rotator Structure (by ref)"))
  ;[1 0.8829 0.4471] HANDLING A NEW PLAYER LOCATION AND ROTATION EVENT
  (if (not (`/Game/Blueprints/MyPlayerController.PlayerControllerHMDCheck` (`self.PlayerController`)))
    (`/Game/ThirdPersonBP/Blueprints/playerPawn.OnReceivedPlayerRotation` (`self.MyPlayerPawn`) Rotation)))

(event `On Player Custom Properties changed` :!signature `self.OnPlayerCustomPropertiesChanged`
  (params (PlayerNumber :type Integer) (ChangedProperties :type "PhotonJSON Object Reference"))
  ;[1 0.651 0.9664] GET PLAYER PROPERTIES
  (set `self.Changed Properties` ChangedProperties))

(event `On Player Color Changed` :!signature `self.OnPlayerColorChanged`
  (params (PlayerNumber :type Integer) (color :type "Color Structure"))
  ;[0.2314 0.2677 1] PLAYER COLOR
  (if true
    _))

(event `Received Player Data Event` :!signature `self.OnReceivedPlayerData`
  (params (PlayerNumber :type Integer) (DataJSON :type "PhotonJSON Object Reference"))
  ;[0.2456 1 0.5543] PLAYER DATA -not properties-
  (if (== (`self.GetPlayerNumber`) (`PhotonJSON.GetInteger` DataJSON "PlayerKicked"))
    (`self.CustomLeaveRoom`)))

(event `On Custom Room Properties Arrive` :!signature `self.OnReceivedChangedCustomRoomProperties`
  (params (ChangedProperties :type "PhotonJSON Object Reference"))
  (bind _returnvalue (`PhotonJSON.GetString` ChangedProperties "mapName"))
  (bind _playercontroller (`self.PlayerController`))
  (bind _playercontroller_2 (`self.PlayerController`))
  (bind (_asigame_mode_change_bp _bsuccess) (cast `/Game/Blueprints/IGameModeChange_BP` (`self.PlayerController`) :!pure true))
  ;[1 0.1354 0.9827] ROOM PROPERTIES INCOMING FROM PHOTON -> change level when master changes it
  (for _array_element (`PhotonJSON.GetKeys` ChangedProperties)
    (`KismetSystemLibrary.PrintString` null _array_element true true (struct :`R` 0.967875 :`G` 1.0 :`A` 1.0) 5.0)
    (switch `string` _array_element
      (:`VideoName`
        (bind _returnvalue_2 (`PhotonJSON.GetString` ChangedProperties _array_element))
        (`/Game/Blueprints/MyPlayerController.SetVideoName` (`self.PlayerController`) _returnvalue_2))
      (:`VideoVolume`
        (bind _returnvalue_3 (`PhotonJSON.GetFloat` ChangedProperties _array_element))
        (`/Game/Blueprints/MyPlayerController.SetVideoVolume` _playercontroller _returnvalue_3)
        (`KismetSystemLibrary.PrintString` null (`KismetStringLibrary.Conv_DoubleToString` _returnvalue_3) :!label _label_2))
      (:`AudioTrack`
        (`/Game/Blueprints/MyPlayerController.SetAudioTrack` _playercontroller _returnvalue_2))
      (:`MusicVolume`
        (`/Game/Blueprints/MyPlayerController.SetMusicVolume` _playercontroller _returnvalue_3)
        (goto _label_2))
      (:`MenuScroll`
        (`/Game/Blueprints/MyPlayerController.SetMenuScroll` _playercontroller _returnvalue_3))
      (:`CGICollapse`
        (`/Game/Blueprints/MyPlayerController.SetCGICollapse` _playercontroller (`PhotonJSON.GetBoolean` ChangedProperties _array_element)))
      (:`MapName`
        (if (and (`KismetSystemLibrary.DoesImplementInterface` (`self.PlayerController`) "/Game/Blueprints/IGameModeChange_BP.IGameModeChange_BP_C") _bsuccess)
          (switch `string` _returnvalue
            (:`Default`
              (`/Game/Blueprints/MyPlayerController.SetMusicVolume` _playercontroller_2 (`PhotonJSON.GetFloat` ChangedProperties "MusicVolume") :!label _label_3)
              (`/Game/Blueprints/MyPlayerController.ShowLoadingScreen` _playercontroller_2))
            (:`LobbyMap`
              _)
            (:`360Map`
              (`/Game/Blueprints/MyPlayerController.SetVideoVolume` _playercontroller_2 (`PhotonJSON.GetFloat` ChangedProperties "VideoVolume"))
              (goto _label_3)))
          (set `self.GameMode` (`PhotonJSON.GetInteger` ChangedProperties "GameMode"))
          (for _array_element_2 (`self.GetRoomPlayers`)
            (`self.MovePlayerPawnToStart` (`.Number` (break `RoomPlayer` _array_element_2))))
          (`/Game/Blueprints/IGameModeChange_BP.ChangeLevelMap` _asigame_mode_change_bp _returnvalue))))))

(event `Clear Players`
  ;[1 1 1] DESTROY PLAYERS
)

(event `Reset Game`
  ;[1 1 1] RESET GAME
  (`self.Clear Players`)
  (`/Game/Blueprints/MyPlayerController.ResetGame` (`self.PlayerController`)))

(event `On Room List Arrives` :!signature `self.OnUpdateRoomList`
  (params (RoomList :type "Array of String (by ref)"))
  ;[1 1 1] ROOM NAMES LIST INCOMING FROM PHOTON
  (if (`/Game/Blueprints/MyPlayerController.PlayerControllerHMDCheck` (`self.PlayerController`))
    (`/Engine/EditorBlueprintResources/StandardMacros.IsValid` (`self.MainMenuUI`)
      (:`Is Valid`
        (`/Game/Blueprints/MyPlayerController.Join Friends Game` (`self.PlayerController`))))))

(event `MovePlayerPawnToStart`
  (params (PlayerNumber :type Integer))
  (bind (_start_location _start_rotation) (`self.GetPlayerStartPoint` PlayerNumber))
  ;[1 1 1] Reset players pawn to the start position
  (`Actor.K2_SetActorLocationAndRotation` (`self.MyPlayerPawn`) _start_location _start_rotation false true))

(event `OnMasterChanged_Func` :!signature `self.OnMasterChanged`
  (params (OldMasterPlayerNumber :type Integer) (NewMasterPlayerNumber :type Integer))
  (`KismetSystemLibrary.PrintString` null "Master Changed" true true (struct :`R` 1.0 :`A` 1.0) 5.0)
  (`/Game/Blueprints/MyPlayerController.ShowCloseGameDialog` (`self.PlayerController`)))

(event `Get Regions Pings`
  (bind _returnvalue (`self.GetPhotonCloudConfig`))
  ;[1 1 1] Get regions pings - new method
  (add `self.OnReceivedPingServersResponse` (delegate `Got Ping Responses`))
  (set `PhotonCloudConfig.regionSelectionMode` "SELECT" _returnvalue)
  (set `PhotonCloudConfig.regionName` "eu" _returnvalue)
  (`self.SelectRegion` "eu")
  (add `self.OnReceivedAvailableRegionsServers` (delegate `Get Available Regions`)))

(event `Get Available Regions` :!signature `self.OnReceivedAvailableRegionsServers`
  (params (availableRegions :type "Array of String (by ref)") (availableRegionsServers :type "Array of String (by ref)"))
  ;[1 1 1] Get regions pings - new method
  (`self.PingServers` availableRegionsServers))

(event `Got Ping Responses` :!signature `self.OnReceivedPingServersResponse`
  (params (PingsResults :type "Array of PingResult Structure (by ref)"))
  ;[1 1 1] Get regions pings - new method
  (for _array_element PingsResults
    (`KismetSystemLibrary.PrintString` self (`KismetStringLibrary.Concat_StrStr` "Server : " (break `PingResult` _array_element)))
    (for _array_element_2 (`.Pings` (break `PingResult` _array_element))
      (`KismetSystemLibrary.PrintString` self (`KismetStringLibrary.Conv_IntToString` _array_element_2)))))

(event `ResetKilledPawn`
  (params (PlayerNumber :type Integer))
  ;[1 1 1] Reset players pawn when if it falls off the map
)

(event `CharacterKilled`
  (params (Key :type "Integer (by ref)")))

(fn `CanWeStart`
  (returns (CanWeStart :type Boolean))
  (locals (LocalStartBool :type Boolean))
  (for _array_element (`self.GetRoomPlayers`)
    (bind (_number _userid _name _customproperties _bisinactive _bismasterclient) (break `RoomPlayer` _array_element))
    (if _bismasterclient
      (set `local.LocalStartBool` true)
      (elif (`KismetStringLibrary.EqualEqual_StrStr` (`PhotonJSON.GetString` _customproperties "ReadyStatus") "Ready")
        (set `local.LocalStartBool` true)
        (else
          (set `local.LocalStartBool` false)
          (break)))))
  (return (`local.LocalStartBool`)))

(fn `GetPlayerStartPoint`
  (params (`Player Number` :type Integer))
  (returns (`Start Location` :type "Vector Structure") (`Start Rotation` :type "Rotator Structure"))
  (locals (StartPoint :type "Transform Structure") (Starts :type "Array of PlayerStart Object Reference"))
  (bind _returnvalue (- `Player Number` 1))
  (bind (_startpoint_location _startpoint_rotation) (`KismetMathLibrary.BreakTransform` (`local.StartPoint`)))
  (bind _returnvalue_2 (`KismetArrayLibrary.Array_Length` (`local.Starts`)))
  (bind _output_get (set `local.Starts` (`/Game/Blueprints/MyPlayerController.GetPlayerStarts` (`self.PlayerController`))))
  (if (`KismetArrayLibrary.Array_IsValidIndex` _output_get _returnvalue)
    (set `local.StartPoint` (`Actor.GetTransform` (`|GetArrayItem` _output_get _returnvalue)))
    (elif (> _returnvalue_2 0)
      (set `local.StartPoint` (`Actor.GetTransform` (`|GetArrayItem` (`local.Starts`) (`KismetMathLibrary.RandomIntegerInRange` 0 (- _returnvalue_2 1)))))))
  (return _startpoint_location _startpoint_rotation))